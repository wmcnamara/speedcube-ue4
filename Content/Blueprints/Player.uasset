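; Player Blueprint for a lane-runner style character that constantly moves forward along X at a frame-rate-independent MovementSpeed.
; MoveLeft and MoveRight input actions shift the Cube component sideways by a fixed step, without sweeping, while the actor itself advances each Tick.
; On overlap, it sends OnPlayerCollisionMessage to the other actor, passing itself so that actor handles the collision response.
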(event Collision|EventActorBeginOverlap
  (params (OtherActor :type Actor%20Object%20Reference))
  ;[1 1 1] Invoke OnPlayerCollision on any object hitting the player
  (if true
    (Class|PlayerInteractable|OnPlayerCollision(Message) OtherActor self)))

(event EventTick
  (params (DeltaSeconds :type Float%20%28single-precision%29))
  ;[1 1 1] Moves the player forward at a constant rate
  (bind _movementvector (CallFunction|GetStaticMovementVector))
  (Transformation|AddRelativeLocation (Variables|Default|GetPlayer) _movementvector false false))

(event Input|ActionEvents|InputActionMoveRight
  (params (Key :type Key%20Structure))
  ;[1 1 1] Input Events
  (:Pressed
    (CallFunction|MoveRight)))

(event Input|ActionEvents|InputActionMoveLeft
  (params (Key :type Key%20Structure))
  ;[1 1 1] Input Events
  (:Pressed
    (CallFunction|MoveLeft)))

(fn ConstructionScript)

(fn MoveLeft
  (Transformation|AddRelativeLocation (Variables|Default|GetCube) "0.000000,-230.000000, 0" false false))

(fn MoveRight
  (Transformation|AddRelativeLocation (Variables|Default|GetCube) "0,230.000000, 0" false false))

(fn GetStaticMovementVector
  (return (Math|Vector|MakeVector (* (Utilities|Time|GetWorldDeltaSeconds) (Variables|Default|GetmovementSpeed)) 0.0 0.0)))